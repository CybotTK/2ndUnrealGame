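; Thunderstorm actor that loops lightning strikes at random intervals of a few seconds, each followed by a brief screen flash and a 2D thunder sound.
; Each strike moves the actor far ahead of the player's view, yaws it by the player's direction and picks one of two bolt textures.
; A timeline animates the plane material's Y and emission, while the flash briefly raises the post-process volume's manual exposure compensation.
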(event Custom|Strike
  (bind _thunder_plane (Variables|Default|GetThunder_Plane))
  (|RelocateThunder
    (:OutputPin
      (|ChangeTexture
        (:OutputPin
          (bind _y (Timeline|Thunder_Strike PlayFromStart)
            (:Update
              (Rendering|Material|SetScalarParameterValueonMaterials _thunder_plane "Y" _y)
              (Rendering|Material|SetScalarParameterValueonMaterials _thunder_plane "emission" (* (+ _y 1.0) 5e+01)))))))))

(event EventBeginPlay
  (bind _pp_volume (Variables|Default|GetPP_Volume))
  (Variables|/Script/Engine.PostProcessVolume|SetSettings (Variables|Default|GetPP_Volume) (Utilities|Struct|MakePostProcessSettings "AEM_Manual" 1e+01))
  (Utilities|FlowControl|Delay (Math|Random|RandomFloatinRange 4.0 8.0) :!label _label)
  (CallFunction|Strike)
  (Utilities|FlowControl|Delay 0.2)
  (bind _output_get (Variables|Default|SetOriginal%20Exposure%20Compensation (Utilities|Struct|BreakPostProcessSettings (Variables|/Script/Engine.PostProcessVolume|GetSettings _pp_volume))))
  (Variables|/Script/Engine.PostProcessVolume|SetSettings _pp_volume (Utilities|Struct|MakePostProcessSettings "AEM_Manual" 12.0))
  (Utilities|FlowControl|Delay 0.1)
  (Variables|/Script/Engine.PostProcessVolume|SetSettings _pp_volume (Utilities|Struct|MakePostProcessSettings "AEM_Manual" _output_get))
  (Audio|PlaySound2D "/Game/Audio/Thunder.Thunder" 1.0 1.0 0.0 0 0)
  (goto _label))

(fn ConstructionScript)